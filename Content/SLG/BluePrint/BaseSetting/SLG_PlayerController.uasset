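; Player controller for the SLG mode, switching between an overhead camera pawn and third-person control of a selected unit.
; Tick and left-mouse input branch on controller and camera state, driving HUD-based selection or cursor-traced placement that spawns units.
; Mode changes blend the view target, then possess the new pawn after a matching delay, guarded by blend flags.
; It also forwards UI states and a looping one-second countdown to the HUD through message interfaces.
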(event `/Game/SLG/BluePrint/BaseSetting/BPI_PlayerController.SetUIByController`
  (params (UIState :type "/Game/SLG/UI/UI_Base/EBP_UIStates Enum" :default "NewEnumerator0"))
  (bind _returnvalue (`self.GetHUD` self))
  ;[1 1 1] 通过Controller控制UI显示状态
  (`/Engine/EditorBlueprintResources/StandardMacros.IsValid` _returnvalue
    (:`Is Valid`
      (bind _ui_base (message `/Game/SLG/BluePrint/BaseSetting/BPI_HUD.CastToUIBase` _returnvalue))
      (`/Engine/EditorBlueprintResources/StandardMacros.IsValid` _ui_base
        (:`Is Valid`
          (`/Game/SLG/UI/UI_Base/UI_Base.SetUIStates` _ui_base UIState))))))

(event `PossessChangeEvent`
  (params (Delay :type "Float (double-precision)") (Pawn :type "Pawn Object Reference"))
  ;[1 1 1] 切换角色
  (`KismetSystemLibrary.Delay` Delay)
  (`self.Possess` Pawn)
  (`|ExecutionSequence`
    (:`then_0`
      (set `self.IsBlendToThirdPerson` false))
    (:`then_1`
      (set `self.IsBlendToCamera` false))))

(event `self.ReceiveBeginPlay`
  ;[1 1 1] BeginPlay
  (`self.InitSetting`))

(event `Key|LeftMouseButton`
  (params (Key :type "Key Structure"))
  (bind _controllerstate (`self.ControllerState`))
  ;[1 1 1] LeftMouseButton
  (:`Pressed`
    (switch `/Game/SLG/BluePrint/BaseSetting/EBP_ControllerState` _controllerstate
      (:`NewEnumerator1`
        (switch `/Game/SLG/BluePrint/BaseSetting/EBP_CameraState` (`self.CameraState`)
          (:`NewEnumerator0`
            (`self.StartSelection`))
          (:`NewEnumerator1`
            (`self.PlacementLeftMouseEvent`))))))
  (:`Released`
    (switch `/Game/SLG/BluePrint/BaseSetting/EBP_ControllerState` _controllerstate
      (:`NewEnumerator1`
        (switch `/Game/SLG/BluePrint/BaseSetting/EBP_CameraState` (`self.CameraState`)
          (:`NewEnumerator0`
            (`self.StopSelection`)))))))

(event `self.ReceiveTick`
  (params (DeltaSeconds :type "Float (single-precision)"))
  ;[1 1 1] TickEvent
  (switch `/Game/SLG/BluePrint/BaseSetting/EBP_ControllerState` (`self.ControllerState`)
    (:`NewEnumerator1`
      (`self.CameraTickEvent`)
      (switch `/Game/SLG/BluePrint/BaseSetting/EBP_CameraState` (`self.CameraState`)
        (:`NewEnumerator0`
          (`self.SelectTick`))
        (:`NewEnumerator1`
          (`self.PlacementTick`))))
    (:`NewEnumerator0`
      (`self.ThirdPersonTickEvent`))))

(event `ActiveTimeEvent`
  (bind _returnvalue (`KismetSystemLibrary.K2_SetTimerDelegate` (delegate `RemaingingLoopEvent`) 1.0 true))
  (set `self.RemainingTimerHandle` _returnvalue))

(event `RemaingingLoopEvent`
  (bind _returnvalue (`self.GetHUD` self))
  (if (>= (`self.RemainingTime`) 0)
    (`/Engine/EditorBlueprintResources/StandardMacros.IsValid` _returnvalue
      (:`Is Valid`
        (bind _ui_base (message `/Game/SLG/BluePrint/BaseSetting/BPI_HUD.CastToUIBase` _returnvalue))
        (`/Engine/EditorBlueprintResources/StandardMacros.IsValid` _ui_base
          (:`Is Valid`
            (bind _ui_timer (message `/Game/SLG/UI/UI_Base/BPI_UI_Base.CastToTimer` _ui_base))
            (`/Engine/EditorBlueprintResources/StandardMacros.IsValid` _ui_timer
              (:`Is Valid`
                (message `/Game/SLG/UI/UI_Timer/BPI_UI_Timer.UpdateRemainingTime` _ui_timer (`KismetTextLibrary.Conv_IntToText` (`self.RemainingTime`)))
                (`/Engine/EditorBlueprintResources/StandardMacros.DecrementInt` (`self.RemainingTime`))))))))
    (else
      (`KismetSystemLibrary.K2_ClearAndInvalidateTimerHandle` (`self.RemainingTimerHandle`)))))

(fn `AddUnitToSelection`
  (params (UnitBase :type "/Game/SLG/BluePrint/Character/BP_Unit_Base Object Reference") (IsSelected :type Boolean))
  (`KismetArrayLibrary.Array_AddUnique` (`self.UnitSelection`) UnitBase)
  (`/Game/SLG/BluePrint/Character/BP_Unit_Base.IsSelected` UnitBase IsSelected))

(fn `CameraTickEvent`
  (bind _bp_camera_pawn (`self.BP Camera Pawn`))
  (bind _bp_camera_pawn_2 (`self.BP Camera Pawn`))
  (if (== (`self.K2_GetPawn`) "/Game/SLG/BluePrint/BaseSetting/BP_CameraPawn.BP_CameraPawn")
    (if (not (`self.bShowMouseCursor`))
      (set `self.bShowMouseCursor` true))
    (elif (not (`self.IsBlendToCamera`))
      (bind _output_get (set `self.CurPawnTransform` (`self.GetTransform` (`self.K2_GetPawn`))))
      (`/Engine/EditorBlueprintResources/StandardMacros.IsValid` _bp_camera_pawn
        (:`Is Valid`
          (`self.K2_SetActorLocationAndRotation` _bp_camera_pawn (.location _output_get) (.rotation _output_get) false false)
          (`self.SetViewTargetWithBlend` _bp_camera_pawn_2 1.0)
          (set `self.IsBlendToCamera` true)
          (`self.PossessChangeEvent` 1.0 _bp_camera_pawn_2))))))

(fn `ClearSelection`
  (for _array_element (`self.UnitSelection`)
    (`/Game/SLG/BluePrint/Character/BP_Unit_Base.IsSelected` _array_element false))
  (`KismetArrayLibrary.Array_Clear` (`self.UnitSelection`)))

(fn `InitSetting`
  (`|ExecutionSequence`
    (:`then_0`
      (set `self.ControllerState` "NewEnumerator1"))
    (:`then_1`
      (set `self.bShowMouseCursor` true)
      (`WidgetBlueprintLibrary.SetInputMode_GameAndUIEx` self null "DoNotLock" false))
    (:`then_2`
      (bind _asbp_camera_pawn (cast `/Game/SLG/BluePrint/BaseSetting/BP_CameraPawn` (`self.GetViewTarget` self))
        (:`then`
          (set `self.BP Camera Pawn` _asbp_camera_pawn))
        (:`CastFailed`
          (`KismetSystemLibrary.PrintString` "CastFailed_BP_CameraPawn"))))
    (:`then_3`
      (bind _returnvalue (`GameplayStatics.GetActorOfClass` "/Game/SLG/BluePrint/Placement/BP_Placement.BP_Placement_C"))
      (`/Engine/EditorBlueprintResources/StandardMacros.IsValid` _returnvalue
        (:`Is Valid`
          (set `self.BP_Placement` _returnvalue))
        (:`Is Not Valid`
          (`KismetSystemLibrary.PrintString` "NoFuondBP_Placement"))))
    (:`then_4`
      (set `self.UIStates` "NewEnumerator0"))
    (:`then_5`
      (set `self.RemainingTime` 99))))

(fn `PlacementLeftMouseEvent`
  (`|ExecutionSequence`
    (:`then_0`
      (set `self.CameraState` "NewEnumerator0"))
    (:`then_1`
      (`|SpawnActorFromClass` "/Game/SLG/BluePrint/Character/BP_Unit_Base.BP_Unit_Base_C" (`KismetMathLibrary.MakeTransform` (+ (`.Location` (`GameplayStatics.BreakHitResult` (`self.Hit Result`))) (0.0 0.0 100.0))) "Undefined" "OverrideRootScale" null null))))

(fn `PlacementTick`
  (bind (_hitresult _returnvalue) (`self.GetHitResultUnderCursorByChannel` "TraceTypeQuery2"))
  (bind _bp_placement (`self.BP_Placement`))
  (if _returnvalue
    (bind _output_get (set `self.Hit Result` _hitresult))
    (`/Engine/EditorBlueprintResources/StandardMacros.IsValid` _bp_placement
      (:`Is Valid`
        (`self.SetActorHiddenInGame` _bp_placement false)
        (`self.K2_SetActorLocation` _bp_placement (`.Location` (`GameplayStatics.BreakHitResult` _output_get)) false false)))))

(fn `RemoveUnitToSelection`
  (params (UnitBase :type "/Game/SLG/BluePrint/Character/BP_Unit_Base Object Reference") (IsSelected :type Boolean))
  (`KismetArrayLibrary.Array_RemoveItem` (`self.UnitSelection`) UnitBase)
  (`/Game/SLG/BluePrint/Character/BP_Unit_Base.IsSelected` UnitBase IsSelected))

(fn `SelectTick`
  (bind _bp_placement (`self.BP_Placement`))
  (`|ExecutionSequence`
    (:`then_0`
      (`/Engine/EditorBlueprintResources/StandardMacros.IsValid` _bp_placement
        (:`Is Valid`
          (`self.SetActorHiddenInGame` _bp_placement true))))))

(fn `StartSelection`
  (message `/Game/SLG/BluePrint/BPI/BPI_MouseSelect.StartSelection` (`self.GetHUD`))
  (if (not (`.ReturnValue` (`self.GetHitResultUnderCursorByChannel` "TraceTypeQuery3")))
    (`self.ClearSelection`)))

(fn `StopSelection`
  (message `/Game/SLG/BluePrint/BPI/BPI_MouseSelect.StopSelection` (`self.GetHUD`)))

(fn `ThirdPersonTickEvent`
  (if (== (`self.K2_GetPawn`) "/Game/SLG/BluePrint/Character/BP_Unit_Base.BP_Unit_Base")
    (if (`self.bShowMouseCursor`)
      (set `self.bShowMouseCursor` false))
    (elif (not (`self.IsBlendToThirdPerson`))
      (for _array_element (`self.UnitSelection`)
        (`/Engine/EditorBlueprintResources/StandardMacros.IsValid` _array_element
          (:`Is Valid`
            (`self.SetViewTargetWithBlend` _array_element 1.0)
            (set `self.IsBlendToThirdPerson` true)
            (`self.EnableInput` _array_element self)
            (`/Game/SLG/BluePrint/Character/BPI_UnitBase.UpdateUnitMoveValue` _array_element)
            (`self.PossessChangeEvent` 1.0 _array_element)
            (break))))
      (`self.ClearSelection`))))

(fn `UserConstructionScript`)