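; HUD Blueprint for an SLG (strategy) game that creates the main UI and handles drag-box selection of units.
; On BeginPlay it creates the UI_Base widget for the SLG player controller and adds it to the viewport.
; While selection is active, DrawHUD draws a rectangle to the DPI-scaled mouse position and, beyond a small drag threshold, gathers units inside it.
; StopSelection then replaces the controller's selection with those units, marking them active.
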(event `self.ReceiveBeginPlay`
  (bind _asslg_player_controller (cast `/Game/SLG/BluePrint/BaseSetting/SLG_PlayerController` (`GameplayStatics.GetPlayerController` 0)))
  (bind _output_get (set `self.SLG Player Controller` _asslg_player_controller))
  (`/Engine/EditorBlueprintResources/StandardMacros.IsValid` _output_get
    (:`Is Valid`
      (bind _returnvalue (`|CreateWidget` "/Game/SLG/UI/UI_Base.UI_Base_C" _output_get _output_get))
      (bind _output_get_2 (set `self.UI_Base` _returnvalue))
      (`UserWidget.AddToViewport` _output_get_2 0))))

(event `/Game/SLG/BluePrint/BPI/BPI_MouseSelect.StartSelection`
  (bind _returnvalue (`WidgetLayoutLibrary.GetMousePositionOnViewport`))
  (bind (_returnvalue_x _returnvalue_y) (`KismetMathLibrary.BreakVector2D` (* _returnvalue (`WidgetLayoutLibrary.GetViewportScale`))))
  (set `self.PointA` (`KismetMathLibrary.MakeVector2D` _returnvalue_x _returnvalue_y))
  (set `self.IsDrawing` true))

(event `/Game/SLG/BluePrint/BPI/BPI_MouseSelect.StopSelection`
  (set `self.IsDrawing` false)
  (if (`self.IsMarquee`)
    (`/Game/SLG/BluePrint/BaseSetting/SLG_PlayerController.ClearSelection` (`self.SLG Player Controller`))
    (for _array_element (`self.SelectionOfActors`)
      (bind _asbp_unit_base (cast `/Game/SLG/BluePrint/Character/BP_Unit_Base` _array_element))
      (bind _output_get (set `/Game/SLG/BluePrint/Character/BP_Unit_Base.IsActive` true _asbp_unit_base))
      (`/Game/SLG/BluePrint/BaseSetting/SLG_PlayerController.AddUnitToSelection` (`self.SLG Player Controller`) _asbp_unit_base _output_get))
    (set `self.IsMarquee` false)))

(event `self.ReceiveDrawHUD`
  (params (SizeX :type Integer) (SizeY :type Integer))
  (bind (_pointa_x _pointa_y) (`KismetMathLibrary.BreakVector2D` (`self.PointA`)))
  (bind (_pointb_x _pointb_y) (`KismetMathLibrary.BreakVector2D` (`self.PointB`)))
  (if (`self.IsDrawing`)
    (bind _returnvalue (`WidgetLayoutLibrary.GetMousePositionOnViewport`))
    (bind (_returnvalue_x _returnvalue_y) (`KismetMathLibrary.BreakVector2D` (* _returnvalue (`WidgetLayoutLibrary.GetViewportScale`))))
    (set `self.PointB` (`KismetMathLibrary.MakeVector2D` _returnvalue_x _returnvalue_y))
    (`self.DrawRect` self (struct :`G` 0.970513 :`B` 1.0 :`A` 0.5) _pointa_x _pointa_y (- _pointb_x _pointa_x) (- _pointb_y _pointa_y))
    (if (> (`KismetMathLibrary.VSize2D` (- (`self.PointA`) (`self.PointB`))) 50.0)
      (set `self.IsMarquee` true)
      (set `self.SelectionOfActors` (`self.GetActorsInSelectionRectangle` "/Game/SLG/BluePrint/Character/BP_Unit_Base.BP_Unit_Base_C" (`self.PointA`) (`self.PointB`) false)))))

(fn `UserConstructionScript`)