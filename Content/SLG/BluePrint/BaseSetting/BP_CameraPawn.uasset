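; Player camera pawn for the SLG (strategy) game, with a spring arm and FInterpTo-smoothed controls.
; Input axes drive pan, yaw and wheel zoom; holding the rotate action turns zoom into arm pitch, and R resets camera values.
; Tick scales speeds by zoom, runs screen-edge scrolling, and adjusts height from a cursor trace, rising at walls, following ground and ignoring units.
; CheckViewStuck is an empty stub.
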(event `self.ReceiveBeginPlay`
  ;[1 1 1] BeginPlay
  (`self.InitSetting`)
  (`self.ReSetCameraStates`))

(event `self.ReceiveTick`
  (params (DeltaSeconds :type "Float (single-precision)"))
  ;[1 1 1] TickEvent
  (set `self.Delta Seconds` DeltaSeconds)
  (`self.ResetSpeed_ZoomFactor`)
  (`|ExecutionSequence`
    (:`then_0`
      (`self.Mouse Movement`))
    (:`then_1`
      (`self.HeightMovement`))
    (:`then_2`
      (`self.CheckViewStuck`))))

(event `InputAxis|MoveForward`
  (params (AxisValue :type "Float (single-precision)"))
  ;[1 1 1] 相机移动
  ;;[1 1 1] W ＆ S 镜头前进后退
  (bind _output_get (set `self.CurrentMoveForward` (`KismetMathLibrary.FInterpTo` (`self.CurrentMoveForward`) (* AxisValue (`self.BaseMoveSpeed`)) (`self.Delta Seconds`) (`self.MoveInterpSpeed`))))
  (`self.AddMovementInput` self (`self.GetActorForwardVector` self) _output_get false))

(event `InputAxis|MoveRight`
  (params (AxisValue :type "Float (single-precision)"))
  (bind _returnvalue (`KismetMathLibrary.FInterpTo` (`self.CurrentlyMoveRight`) (* AxisValue (`self.BaseMoveSpeed`)) (`self.Delta Seconds`) (`self.MoveInterpSpeed`)))
  ;[1 1 1] 相机移动
  ;;[1 1 1] A ＆ D 镜头左右平移
  (set `self.CurrentlyMoveRight` _returnvalue)
  (`self.AddMovementInput` self (`self.GetActorRightVector` self) _returnvalue false))

(event `InputAxis|TurnCamera`
  (params (AxisValue :type "Float (single-precision)"))
  ;[1 1 1] 相机移动
  ;;[1 1 1] Q ＆ E 镜头左右旋转
  (bind _output_get (set `self.CurrentlyTurnCamera` (`KismetMathLibrary.FInterpTo` (`self.CurrentlyTurnCamera`) (* AxisValue (`self.BaseTurnSpeed`)) (`self.Delta Seconds`) (`self.TurnInterpSpeed`))))
  (`self.AddControllerYawInput` self _output_get))

(event `Key|R`
  (params (Key :type "Key Structure"))
  ;[1 1 1] 相机移动
  (:`Pressed`
    (`self.ReSetCameraStates`)))

(event `InputAction|ActiveRotatedCamera`
  (params (Key :type "Key Structure"))
  ;[1 1 1] 相机移动
  ;;[1 1 1] 鼠标右键激活旋转相机
  (:`Pressed`
    (set `self.IsActiveRotatedCamera` true))
  (:`Released`
    (set `self.IsActiveRotatedCamera` false)))

(event `InputAxis|ZoomCamera`
  (params (AxisValue :type "Float (single-precision)"))
  ;[1 1 1] 相机移动
  ;;[1 1 1] 滚轮缩放镜头摇臂
  (if (not (`self.IsActiveRotatedCamera`))
    (bind _output_get (set `self.BaseSpringArmLength` (`KismetMathLibrary.FInterpTo` (`self.BaseSpringArmLength`) (`KismetMathLibrary.FClamp` (+ (* AxisValue (`self.ZoomFactor`) 100.0 -1.0) (`self.BaseSpringArmLength`)) 300.0 2000.0) (`self.Delta Seconds`) (`self.ZoomInterpSpeed`))))
    (set `SpringArmComponent.TargetArmLength` _output_get (`self.SpringArm`))))

(event `InputAxis|RotatedCamera`
  (params (AxisValue :type "Float (single-precision)"))
  (bind _springarm (`self.SpringArm`))
  (bind (_relativerotation_roll _relativerotation_pitch _relativerotation_yaw) (`KismetMathLibrary.BreakRotator` (`SceneComponent.RelativeRotation` _springarm)))
  ;[1 1 1] 相机移动
  ;;[1 1 1] 右键+滚轮调整摇臂角度
  (if (`self.IsActiveRotatedCamera`)
    (bind _output_get (set `self.CameraArmAngle` (`KismetMathLibrary.FInterpTo` (`self.CameraArmAngle`) (`KismetMathLibrary.ClampAngle` (+ (* AxisValue (`self.CameraRotatedSpeed`)) (`self.CameraArmAngle`)) -75.0 -15.0) (`self.Delta Seconds`) (`self.CameraRotatedInterpSpeed`))))
    (`SceneComponent.K2_SetRelativeRotation` _springarm (`KismetMathLibrary.MakeRotator` _relativerotation_roll _output_get _relativerotation_yaw) false false)))

(fn `CheckViewStuck`)

(fn `HeightMovement`
  (bind (_hitresult _returnvalue) (`PlayerController.GetHitResultUnderCursorByChannel` (`self.SLG Player Controller`) "TraceTypeQuery4" true))
  (bind (_bblockinghit _binitialoverlap _time _distance _location _impactpoint _normal _impactnormal _physmat _hitactor) (`GameplayStatics.BreakHitResult` _hitresult))
  (bind _returnvalue_2 (- (.z (`.Location` (`GameplayStatics.BreakHitResult` _hitresult))) (.z (`self.K2_GetActorLocation` self))))
  ;[1 1 1] 检测射线射到墙壁的时候上升
  (if _returnvalue
    (cast `/Game/SLG/BluePrint/Character/BP_Unit_Base` _hitactor
      (:`CastFailed`
        (if (or (> (`KismetMathLibrary.Abs` (.x _normal)) 0.9) (> (`KismetMathLibrary.Abs` (.y _normal)) 0.9))
          (bind _output_get (set `self.CurrentlyHeightInput` (`KismetMathLibrary.FInterpTo` (`self.CurrentlyHeightInput`) 1.0 (`self.Delta Seconds`) (`self.HeightInterpSpeed`))))
          (`self.AddMovementInput` self (`self.GetActorUpVector` self) _output_get false)
          (else
            ;[1 1 1] 保证相机根节点贴地
            (if (<= _returnvalue_2 -50.0)
              (bind _output_get_2 (set `self.CurrentlyHeightInput` (`KismetMathLibrary.FInterpTo` (`self.CurrentlyHeightInput`) -1.0 (`self.Delta Seconds`) (`self.HeightInterpSpeed`))))
              (`self.AddMovementInput` self (`self.GetActorUpVector` self) _output_get_2 false)
              (elif (>= _returnvalue_2 50.0)
                (bind _output_get_3 (set `self.CurrentlyHeightInput` (`KismetMathLibrary.FInterpTo` (`self.CurrentlyHeightInput`) 1.0 (`self.Delta Seconds`) (`self.HeightInterpSpeed`))))
                (`self.AddMovementInput` self (`self.GetActorUpVector` self) _output_get_3 false)))))))))

(fn `InitSetting`
  (`|ExecutionSequence`
    (:`then_0`
      (bind _asslg_player_controller (cast `/Game/SLG/BluePrint/BaseSetting/SLG_PlayerController` (`self.GetController` self))
        (:`then`
          (bind _output_get (set `self.SLG Player Controller` _asslg_player_controller))
          (`PlayerController.SetViewTargetWithBlend` _output_get self 0.0 "VTBlend_Linear" 0.0 false)
          (`self.EnableInput` self (`self.SLG Player Controller`)))
        (:`CastFailed`
          (`KismetSystemLibrary.PrintString` "CastFailed_SLG_PlayerController"))))
    (:`then_1`
      (set `self.bUseControllerRotationYaw` true))))

(fn `Mouse Movement`
  (bind (_x _y) (`KismetMathLibrary.BreakVector2D` (/ (`WidgetLayoutLibrary.GetViewportSize`) (`WidgetLayoutLibrary.GetViewportScale`))))
  (bind _returnvalue (`WidgetLayoutLibrary.GetMousePositionOnViewport`))
  (`|ExecutionSequence`
    (:`then_0`
      (bind (_x_2 _y_2) (`KismetMathLibrary.BreakVector2D` _returnvalue))
      ;[1 1 1] MoveForward
      (if (<= _y_2 (`self.MouseMove_GapValue`))
        (bind _output_get (set `self.CurrentlyMouseForward` (`KismetMathLibrary.FInterpTo` (`self.CurrentlyMouseForward`) (`self.BaseMoveSpeed`) (`self.Delta Seconds`) (`self.MoveInterpSpeed`))))
        (`self.AddMovementInput` self (`self.GetActorForwardVector` self) _output_get false)
        (else
          (bind _output_get_2 (set `self.CurrentlyMouseForward` (`KismetMathLibrary.FInterpTo` (`self.CurrentlyMouseForward`) 0.0 (`self.Delta Seconds`) (`self.MoveInterpSpeed`)) :!label _label))
          (`self.AddMovementInput` self (`self.GetActorForwardVector` self) _output_get_2 false))))
    (:`then_1`
      (if (>= _y_2 (- _y (`self.MouseMove_GapValue`)))
        (bind _output_get_3 (set `self.CurrentlyMouseForward` (`KismetMathLibrary.FInterpTo` (`self.CurrentlyMouseForward`) (* (`self.BaseMoveSpeed`) -1.0) (`self.Delta Seconds`) (`self.MoveInterpSpeed`))))
        (`self.AddMovementInput` self (`self.GetActorForwardVector` self) _output_get_3 false)
        (else
          (goto _label))))
    (:`then_2`
      ;[1 1 1] MoveRight
      (if (<= _x_2 (`self.CurrentlyMouseForward`))
        (bind _output_get_4 (set `self.CurrentlyMouseRight` (`KismetMathLibrary.FInterpTo` (`self.CurrentlyMouseRight`) (* (`self.BaseMoveSpeed`) -1.0) (`self.Delta Seconds`) (`self.MoveInterpSpeed`))))
        (`self.AddMovementInput` self (`self.GetActorRightVector` self) _output_get_4 false)
        (else
          (bind _output_get_5 (set `self.CurrentlyMouseRight` (`KismetMathLibrary.FInterpTo` (`self.CurrentlyMouseRight`) 0.0 (`self.Delta Seconds`) (`self.MoveInterpSpeed`)) :!label _label_2))
          (`self.AddMovementInput` self (`self.GetActorRightVector` self) _output_get_5 false))))
    (:`then_3`
      (if (>= _x_2 (- _x (`self.CurrentlyMouseForward`)))
        (bind _output_get_6 (set `self.CurrentlyMouseRight` (`KismetMathLibrary.FInterpTo` (`self.CurrentlyMouseRight`) (`self.BaseMoveSpeed`) (`self.Delta Seconds`) (`self.MoveInterpSpeed`))))
        (`self.AddMovementInput` self (`self.GetActorRightVector` self) _output_get_6 false)
        (else
          (goto _label_2))))))

(fn `ReSetCameraStates`
  (`|ExecutionSequence`
    (:`then_0`
      (set `self.CameraArmAngle` -60.0))
    (:`then_1`
      (set `self.BaseSpringArmLength` 1000.0))))

(fn `ResetSpeed_ZoomFactor`
  (set `self.ZoomFactor` (`KismetMathLibrary.FInterpTo` (`self.ZoomFactor`) (`KismetMathLibrary.FClamp` (/ (`SpringArmComponent.TargetArmLength` (`self.SpringArm`)) (`self.DeafultSpringArmLength`)) 0.3 2.0) (`self.Delta Seconds`) (`self.ZoomInterpSpeed`)))
  (`|ExecutionSequence`
    (:`then_0`
      (set `self.BaseMoveSpeed` (`KismetMathLibrary.FInterpTo` (`self.BaseMoveSpeed`) (+ (* (`self.ZoomFactor`) 5.0) (`self.DefaultMoveSpeed`)) (`self.Delta Seconds`) (`self.MoveInterpSpeed`))))
    (:`then_2`
      (set `self.CameraRotatedSpeed` (`KismetMathLibrary.FInterpTo` (`self.CameraRotatedSpeed`) (+ (* (`self.ZoomFactor`) 1.0) 30.0) (`self.Delta Seconds`) (`self.CameraRotatedInterpSpeed`))))))

(fn `UserConstructionScript`)