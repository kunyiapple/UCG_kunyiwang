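; BP_DecalToWorld is an actor that shows a cursor decal on world surfaces while the player uses the SLG camera pawn mode.
; It caches the SLG player controller on BeginPlay and checks its controller state every tick.
; In Camera Pawn state, a cursor trace places the decal at the hit point, oriented to the surface normal, and reveals it once.
; In Third Person state, it hides the decal and resets that one-time reveal.
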(event `self.ReceiveBeginPlay`
  (bind _asslg_player_controller (cast `/Game/SLG/BluePrint/BaseSetting/SLG_PlayerController` (`GameplayStatics.GetPlayerController` 0)))
  (set `self.SLG Player Controller` _asslg_player_controller))

(event `self.ReceiveTick`
  (params (DeltaSeconds :type "Float (single-precision)"))
  (bind _slg_player_controller (`self.SLG Player Controller`))
  (bind (_bblockinghit _binitialoverlap _time _distance _location _impactpoint _normal _impactnormal) (`GameplayStatics.BreakHitResult` (`PlayerController.GetHitResultUnderCursorByChannel` (`self.SLG Player Controller`) "TraceTypeQuery3" true)))
  (`/Engine/EditorBlueprintResources/StandardMacros.IsValid` _slg_player_controller
    (:`Is Valid`
      (switch `/Game/SLG/BluePrint/BaseSetting/EBP_ControllerState` (`/Game/SLG/BluePrint/BaseSetting/SLG_PlayerController.ControllerState` _slg_player_controller)
        (:`NewEnumerator1`
          (`SceneComponent.K2_SetWorldLocationAndRotation` (`self.DecalToWorld`) _location (`KismetMathLibrary.MakeRotationFromAxes` _impactnormal) false false)
          (`/Engine/EditorBlueprintResources/StandardMacros.DoOnce` false :!label _label
            (:`Completed`
              (`SceneComponent.SetVisibility` (`self.DecalToWorld`) true false))))
        (:`NewEnumerator0`
          (`SceneComponent.SetVisibility` (`self.DecalToWorld`) false false)
          (goto _label :!via `Reset`))))))

(fn `UserConstructionScript`)